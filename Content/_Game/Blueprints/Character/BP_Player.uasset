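; BP_Player is the player character, with a 2D Paper sprite weapon display using DOOM RPG art and simple health handling.
; The MachineGun flag selects between two weapons' sprites in the change-weapon and shoot events.
; Shooting only briefly swaps to a firing sprite before restoring the idle one, with no hit logic here.
; Incoming damage reduces integer Life and opens L_Debug once it is depleted.
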(event `self.ReceiveTick`
  (params (DeltaSeconds :type "Float (single-precision)"))
  (`parent.ReceiveTick` DeltaSeconds))

(event `E_ChangeWeapon`
  (bind _papersprite (`self.PaperSprite`))
  (if (`self.MachineGun`)
    (`PaperSpriteComponent.SetSprite` _papersprite "/Game/_Game/Assets/Animations/Mobile_-_DOOM_RPG_-_Weapons_Sprite_181.Mobile_-_DOOM_RPG_-_Weapons_Sprite_181")
    (else
      (`PaperSpriteComponent.SetSprite` _papersprite "/Game/_Game/Assets/Animations/Mobile_-_DOOM_RPG_-_Weapons_Sprite_149.Mobile_-_DOOM_RPG_-_Weapons_Sprite_149"))))

(event `E_shoot`
  (bind _papersprite (`self.PaperSprite`))
  (bind _papersprite_2 (`self.PaperSprite`))
  (if (`self.MachineGun`)
    (`PaperSpriteComponent.SetSprite` _papersprite_2 "/Game/_Game/Assets/Animations/Mobile_-_DOOM_RPG_-_Weapons_Sprite_231.Mobile_-_DOOM_RPG_-_Weapons_Sprite_231")
    (`KismetSystemLibrary.Delay` 0.1)
    (`PaperSpriteComponent.SetSprite` _papersprite_2 "/Game/_Game/Assets/Animations/Mobile_-_DOOM_RPG_-_Weapons_Sprite_181.Mobile_-_DOOM_RPG_-_Weapons_Sprite_181")
    (else
      (`PaperSpriteComponent.SetSprite` _papersprite "/Game/_Game/Assets/Animations/Mobile_-_DOOM_RPG_-_Weapons_Sprite_100.Mobile_-_DOOM_RPG_-_Weapons_Sprite_100")
      (`KismetSystemLibrary.Delay` 0.1)
      (`PaperSpriteComponent.SetSprite` _papersprite "/Game/_Game/Assets/Animations/Mobile_-_DOOM_RPG_-_Weapons_Sprite_149.Mobile_-_DOOM_RPG_-_Weapons_Sprite_149"))))

(event `self.ReceiveAnyDamage`
  (params (Damage :type "Float (single-precision)") (DamageType :type "DamageType Object Reference") (InstigatedBy :type "Controller Object Reference") (DamageCauser :type "Actor Object Reference"))
  (set `self.Life` (`KismetMathLibrary.FTrunc` (- (`self.Life`) Damage)))
  (if (<= (`self.Life`) 0)
    (`GameplayStatics.OpenLevel` "L_Debug")))

(fn `UserConstructionScript`
  (`parent.UserConstructionScript`))