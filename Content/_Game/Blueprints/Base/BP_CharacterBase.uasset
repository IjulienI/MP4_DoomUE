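; BP_CharacterBase is a base character Blueprint that tracks health for the game's characters.
; Health starts at MaxHealth on BeginPlay, and AnyDamage subtracts the truncated damage amount from it.
; IsDead reports whether Health is at or below zero; the damage event calls it but does nothing with the result.
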(event `self.ReceiveBeginPlay`
  (set `self.Health` (`self.MaxHealth`)))

(event `self.ReceiveAnyDamage`
  (params (Damage :type "Float (single-precision)") (DamageType :type "DamageType Object Reference") (InstigatedBy :type "Controller Object Reference") (DamageCauser :type "Actor Object Reference"))
  (set `self.Health` (- (`self.Health`) (`KismetMathLibrary.FTrunc` Damage)))
  (`self.IsDead?`))

(fn `IsDead?`
  (returns (Death :type Boolean))
  (return (<= (`self.Health`) 0)))

(fn `UserConstructionScript`)