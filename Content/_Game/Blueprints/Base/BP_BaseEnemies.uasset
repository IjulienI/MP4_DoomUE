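; Base enemy actor, a Doom-style billboard sprite that chases the player and deals contact damage.
; Tick turns the flipbook toward the player, picks a directional flipbook from look-at yaw sectors, and activates animation and AI pursuit within range.
; Sphere overlap applies damage to BP_Player behind a delay-reset DoOnce.
; Taking damage lowers health and triggers pursuit; death sets the Cacodemon death flipbook, disables collision, then destroys the actor.
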(event `self.ReceiveBeginPlay`
  (bind _returnvalue (`GameplayStatics.GetActorOfClass` "/Game/_Game/Blueprints/Base/BP_CharacterBase.BP_CharacterBase_C"))
  (set `self.Player` _returnvalue)
  (`PaperFlipbookComponent.SetPlayRate` (`self.PaperFlipbook`) 0.0))

(event `self.ReceiveTick`
  (params (DeltaSeconds :type "Float (single-precision)"))
  (bind _paperflipbook (`self.PaperFlipbook`))
  (bind _paperflipbook_2 (`self.PaperFlipbook`))
  (bind (_returnvalue_roll _returnvalue_pitch _returnvalue_yaw) (`KismetMathLibrary.BreakRotator` (`KismetMathLibrary.FindLookAtRotation` (`SceneComponent.K2_GetComponentLocation` _paperflipbook_2) (`self.K2_GetActorLocation` (`self.Player`)))))
  (`SceneComponent.K2_SetWorldRotation` _paperflipbook_2 (`KismetMathLibrary.MakeRotator` _returnvalue_roll 0.0 (- _returnvalue_yaw 90.0)) false false)
  (`self.SetDirection`)
  (`self.SetFlipBook`)
  (if (`self.active`)
    (`PaperFlipbookComponent.SetPlayRate` _paperflipbook 1.0)
    (else
      (`PaperFlipbookComponent.SetPlayRate` _paperflipbook 0.0)))
  (if (<= (`KismetMathLibrary.Abs` (`KismetMathLibrary.VSize` (- (`self.K2_GetActorLocation` (`self.Player`)) (`self.K2_GetActorLocation`)))) 500.0)
    (set `self.active` true)
    (`|AIMoveTo` self (0.0 0.0 0.0) (`self.Player`)
      (:`then`
        (`self.K2_SetActorRotation` (`KismetMathLibrary.FindLookAtRotation` (`self.K2_GetActorLocation`) (`self.K2_GetActorLocation` (`self.Player`))))))))

(event `self.ReceiveAnyDamage`
  (params (Damage :type "Float (single-precision)") (DamageType :type "DamageType Object Reference") (InstigatedBy :type "Controller Object Reference") (DamageCauser :type "Actor Object Reference"))
  (bind _paperflipbook (`self.PaperFlipbook`))
  (set `self.Health` (- (`self.Health`) (`KismetMathLibrary.FTrunc` Damage)))
  (`|AIMoveTo` self (0.0 0.0 0.0) (`self.Player`)
    (:`then`
      (bind _dead (`self.IsDead?`))
      (if _dead
        (set `self.active` true)
        (`PaperFlipbookComponent.SetPlayRate` _paperflipbook 1.0)
        (`PaperFlipbookComponent.SetFlipbook` _paperflipbook "/Game/_Game/Assets/Animations/FlipBooks/PF_CacodemonDeath.PF_CacodemonDeath")
        (`PrimitiveComponent.SetCollisionEnabled` (`self.Capsule`) "NoCollision")
        (`KismetSystemLibrary.Delay` 2.0)
        (`self.K2_DestroyActor`)))))

(event `self.Sphere.OnComponentBeginOverlap`
  (params (OverlappedComponent :type "PrimitiveComponent Object Reference") (OtherActor :type "Actor Object Reference") (OtherComp :type "PrimitiveComponent Object Reference") (OtherBodyIndex :type Integer) (bFromSweep :type Boolean) (SweepResult :type "HitResult Structure (by ref)"))
  (bind _asbp_player (cast `/Game/_Game/Blueprints/Character/BP_Player` OtherActor))
  (`/Engine/EditorBlueprintResources/StandardMacros.DoOnce` false :!label _label
    (:`Completed`
      (`GameplayStatics.ApplyDamage` _asbp_player 15.0)
      (`KismetSystemLibrary.Delay` 0.5)
      (`self.E_CanTakeDamage`))))

(event `E_CanTakeDamage`
  (goto _label :!via `Reset`))

(fn `IsDead?`
  (returns (Dead :type Boolean))
  (return (<= (`self.Health`) 0)))

(fn `SetDirection`
  (bind (_returnvalue_roll _returnvalue_pitch _returnvalue_yaw) (`KismetMathLibrary.BreakRotator` (`KismetMathLibrary.FindLookAtRotation` (`self.K2_GetActorLocation`) (`self.K2_GetActorLocation` (`self.Player`)))))
  (if (< _returnvalue_yaw 0.0)
    (`/Engine/EditorBlueprintResources/StandardMacros.CompareFloat` _returnvalue_yaw -45.0
      (:`>`
        (set `self.Direction` "NewEnumerator0" :!label _label))
      (:`==`
        (goto _label))
      (:`<`
        (`/Engine/EditorBlueprintResources/StandardMacros.CompareFloat` _returnvalue_yaw -90.0
          (:`>`
            (set `self.Direction` "NewEnumerator5" :!label _label_2))
          (:`==`
            (goto _label_2))
          (:`<`
            (`/Engine/EditorBlueprintResources/StandardMacros.CompareFloat` _returnvalue_yaw -135.0
              (:`>`
                (set `self.Direction` "NewEnumerator3" :!label _label_3))
              (:`==`
                (goto _label_3))
              (:`<`
                (`/Engine/EditorBlueprintResources/StandardMacros.CompareFloat` _returnvalue_yaw -180.0
                  (:`>`
                    (set `self.Direction` "NewEnumerator7" :!label _label_4))
                  (:`==`
                    (goto _label_4))
                  (:`<`
                    (set `self.Direction` "NewEnumerator2" :!label _label_5)))))))))
    (else
      (`/Engine/EditorBlueprintResources/StandardMacros.CompareFloat` _returnvalue_yaw 180.0
        (:`>`
          (set `self.Direction` "NewEnumerator4" :!label _label_6))
        (:`==`
          (goto _label_6))
        (:`<`
          (`/Engine/EditorBlueprintResources/StandardMacros.CompareFloat` _returnvalue_yaw 135.0
            (:`>`
              (goto _label_5))
            (:`==`
              (goto _label_5))
            (:`<`
              (`/Engine/EditorBlueprintResources/StandardMacros.CompareFloat` _returnvalue_yaw 90.0
                (:`>`
                  (set `self.Direction` "NewEnumerator6" :!label _label_7))
                (:`==`
                  (goto _label_7))
                (:`<`
                  (`/Engine/EditorBlueprintResources/StandardMacros.CompareFloat` _returnvalue_yaw 45.0
                    (:`>`
                      _)
                    (:`==`
                      _)
                    (:`<`
                      (goto _label_6)))
                  (set `self.Direction` "NewEnumerator1"))))))))))

(fn `SetFlipBook`
  (`PaperFlipbookComponent.SetFlipbook` (`self.PaperFlipbook`) (`|GetArrayItem` (`self.FlipBooks`) (`KismetMathLibrary.Conv_ByteToInt` (`self.Direction`)))))

(fn `UserConstructionScript`)